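; BP_WorldCapture is a scene capture actor that fits its orthographic view to a world area marked by two corner actors.
; When both corners are valid, the construction script centers the actor between them in X and Y, keeping its current height.
; It sets the capture's OrthoWidth to the larger of the X and Y spans, so framing needs no runtime logic.
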(fn `UserConstructionScript`
  (bind (_returnvalue_x _returnvalue_y _returnvalue_z) (`KismetMathLibrary.BreakVector` (`self.K2_GetActorLocation`)))
  (bind _upperleftcorner (`self.UpperLeftCorner`))
  (bind _lowerrightcorner (`self.LowerRightCorner`))
  (bind (_returnvalue_x_2 _returnvalue_y_2) (`KismetMathLibrary.BreakVector` (`self.K2_GetActorLocation` (`self.UpperLeftCorner`))))
  (bind (_returnvalue_x_3 _returnvalue_y_3) (`KismetMathLibrary.BreakVector` (`self.K2_GetActorLocation` (`self.LowerRightCorner`))))
  (bind _returnvalue (`self.K2_GetActorLocation` _upperleftcorner))
  (bind (_returnvalue_x_4 _returnvalue_y_4) (`KismetMathLibrary.BreakVector` (+ (/ (- (`self.K2_GetActorLocation` _lowerrightcorner) _returnvalue) 2.0) _returnvalue)))
  (`/Engine/EditorBlueprintResources/StandardMacros.IsValid` _upperleftcorner
    (:`Is Valid`
      (`/Engine/EditorBlueprintResources/StandardMacros.IsValid` _lowerrightcorner
        (:`Is Valid`
          (`self.K2_SetActorLocation` (`KismetMathLibrary.MakeVector` _returnvalue_x_4 _returnvalue_y_4 _returnvalue_z) false true)
          (set `SceneCaptureComponent2D.OrthoWidth` (`KismetMathLibrary.FMax` (`KismetMathLibrary.Abs` (- _returnvalue_x_3 _returnvalue_x_2)) (`KismetMathLibrary.Abs` (- _returnvalue_y_3 _returnvalue_y_2))) (`self.SceneCapture`)))))))