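; AC_WorldMap sets up the world map UI for a player and supplies the coordinate math that maps world locations onto it.
; InitializeMap stores a valid player, creates the W_Main widget, passes itself to its WorldMap for initialization and adds it to the viewport.
; Two corner actors define the map bounds, giving width and height and converting locations to absolute offsets from the upper-left, with world Y as map X.
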(event `InitializeMap`
  (params (Player :type "Character Object Reference"))
  (`/Engine/EditorBlueprintResources/StandardMacros.IsValid` Player
    (:`Is Valid`
      (set `self.Player` Player)
      (bind _returnvalue (`|CreateWidget` "/Game/WorldMapAssets/Widgets/W_Main.W_Main_C"))
      (bind _output_get (set `self.MainReference` _returnvalue))
      (bind _output_get_2 (set `self.MapReference` (`/Game/WorldMapAssets/Widgets/W_Main.WorldMap` _output_get)))
      (`/Game/WorldMapAssets/Widgets/W_WorldMap.Initialize` _output_get_2 self)
      (`UserWidget.AddToViewport` (`self.MainReference`) 0))
    (:`Is Not Valid`
      (`KismetSystemLibrary.PrintString` "Error: Player is not valid" true true (struct :`R` 1.0 :`A` 1.0) 3.0))))

(fn `ConvertLocationToMapLocation`
  (params (Location :type "Vector Structure"))
  (returns (MapLocation :type "Vector2D Structure"))
  (bind _returnvalue_x (`KismetMathLibrary.BreakVector` (`Actor.K2_GetActorLocation` (`self.UpperLeftCorner`))))
  (bind (_returnvalue_x_2 _returnvalue_y) (`KismetMathLibrary.BreakVector` (`Actor.K2_GetActorLocation` (`self.UpperLeftCorner`))))
  (return (`KismetMathLibrary.MakeVector2D` (`KismetMathLibrary.Abs` (- Location_Y _returnvalue_y)) (`KismetMathLibrary.Abs` (- Location_X _returnvalue_x)))))

(fn `GetMapHeight`
  (returns (MapHeight :type "Float (double-precision)"))
  (bind _returnvalue_x (`KismetMathLibrary.BreakVector` (`Actor.K2_GetActorLocation` (`self.LowerRightCorner`))))
  (bind _returnvalue_x_2 (`KismetMathLibrary.BreakVector` (`Actor.K2_GetActorLocation` (`self.UpperLeftCorner`))))
  (return (`KismetMathLibrary.Abs` (- _returnvalue_x _returnvalue_x_2))))

(fn `GetMapWidth`
  (returns (MapWidth :type "Float (double-precision)"))
  (bind (_returnvalue_x _returnvalue_y) (`KismetMathLibrary.BreakVector` (`Actor.K2_GetActorLocation` (`self.LowerRightCorner`))))
  (bind (_returnvalue_x_2 _returnvalue_y_2) (`KismetMathLibrary.BreakVector` (`Actor.K2_GetActorLocation` (`self.UpperLeftCorner`))))
  (return (`KismetMathLibrary.Abs` (- _returnvalue_y _returnvalue_y_2))))