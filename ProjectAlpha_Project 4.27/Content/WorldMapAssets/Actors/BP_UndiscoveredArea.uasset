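; World map actor marking an undiscovered area, optionally covered by a smoke particle effect scaled to its radius.
; The construction script sizes an area sphere and a larger discover sphere from the radius settings.
; The first overlap by an actor with an AC_WorldMap component reports the area to that component.
; OnDiscover deactivates the smoke, waits briefly for it to fade, then destroys the actor.
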(event `OnDiscover`
  (bind _particlesystem (`self.ParticleSystem`))
  (`/Engine/EditorBlueprintResources/StandardMacros.IsValid` _particlesystem
    (:`Is Valid`
      (`ActorComponent.Deactivate` _particlesystem)
      (`KismetSystemLibrary.Delay` 3.0))
    (:`Is Not Valid`
      _))
  (`self.K2_DestroyActor`))

(event `self.ReceiveBeginPlay`
  (if (not (`self.ShowSmoke?`))
    (`ActorComponent.K2_DestroyComponent` (`self.ParticleSystem`))))

(event `self.DiscoverSphere.OnComponentBeginOverlap`
  (params (OverlappedComponent :type "PrimitiveComponent Object Reference") (OtherActor :type "Actor Object Reference") (OtherComp :type "PrimitiveComponent Object Reference") (OtherBodyIndex :type Integer) (bFromSweep :type Boolean) (SweepResult :type "HitResult Structure (by ref)"))
  (bind _returnvalue (`self.GetComponentByClass` OtherActor "/Game/WorldMapAssets/Actors/AC_WorldMap.AC_WorldMap_C"))
  (`/Engine/EditorBlueprintResources/StandardMacros.IsValid` _returnvalue
    (:`Is Valid`
      (`/Engine/EditorBlueprintResources/StandardMacros.DoOnce` false
        (:`Completed`
          (`/Game/WorldMapAssets/Actors/AC_WorldMap.OnDiscoverArea` _returnvalue self))))))

(fn `UserConstructionScript`
  (bind _arearadius (`self.AreaRadius`))
  (`SphereComponent.SetSphereRadius` (`self.AreaSphere`) _arearadius false)
  (`SphereComponent.SetSphereRadius` (`self.DiscoverSphere`) (+ _arearadius (`self.AdditionalDiscoverRadius`)) false)
  (`SceneComponent.SetRelativeScale3D` (`self.ParticleSystem`) (`KismetMathLibrary.Conv_DoubleToVector` (`KismetMathLibrary.FClamp` (/ (`self.AreaRadius`) 150.0) 0.1 100.0)))
  (`SceneComponent.SetVisibility` (`self.ParticleSystem`) (`self.ShowSmoke?`) false))