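; Component that runs a toggleable, zoomable world map widget showing the player and clickable markers.
; Two corner actors define world bounds for converting between world and map positions, with zoom rescaling the map and optionally icons.
; Player position refreshes on movement, or by looping timer during jumps while the map is visible.
; Map clicks trace down to spawn BP_Marker actors with paired widgets, recycling colours and removing the oldest at the limit.
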(event `InitializeMap`
  (params (Player :type "Character Object Reference"))
  (bind _mapreference (`self.MapReference`))
  (bind _mapreference_2 (`self.MapReference`))
  (`/Engine/EditorBlueprintResources/StandardMacros.IsValid` Player
    (:`Is Valid`
      (set `self.Player` Player)
      (bind _returnvalue (`|CreateWidget` "/Game/WorldMapAssets/Widgets/W_Main.W_Main_C"))
      (bind _output_get (set `self.MainReference` _returnvalue))
      (bind _output_get_2 (set `self.MapReference` (`/Game/WorldMapAssets/Widgets/W_Main.WorldMap` _output_get)))
      (`/Game/WorldMapAssets/Widgets/W_WorldMap.Initialize` _output_get_2 self)
      (set `self.OriginalPlayerSize` (`KismetMathLibrary.MakeVector2D` (`KismetMathLibrary.Conv_IntToDouble` (`/Game/WorldMapAssets/Widgets/W_WorldMap.PlayerSizeX` _mapreference)) (`KismetMathLibrary.Conv_IntToDouble` (`/Game/WorldMapAssets/Widgets/W_WorldMap.PlayerSizeY` _mapreference))))
      (set `self.OriginalMapSize` (`KismetMathLibrary.MakeVector2D` (`KismetMathLibrary.Conv_IntToDouble` (`/Game/WorldMapAssets/Widgets/W_WorldMap.MapSizeX` _mapreference_2)) (`KismetMathLibrary.Conv_IntToDouble` (`/Game/WorldMapAssets/Widgets/W_WorldMap.MapSizeY` _mapreference_2))))
      (set `self.OriginalMarkerSize` (`self.MarkerSize`))
      (set `self.AvailableColours` (`self.MarkerColours`))
      (`self.ShowMap` false)
      (`UserWidget.AddToViewport` (`self.MainReference`) 0))
    (:`Is Not Valid`
      (`KismetSystemLibrary.PrintString` "Error: Player is not valid" true true (struct :`R` 1.0 :`A` 1.0) 3.0))))

(event `OnPlayerMove`
  (if (`self.Visible?`)
    (`self.UpdatePlayerPositionOnMap`)))

(event `StartTimer`
  (bind _returnvalue (`KismetSystemLibrary.K2_SetTimer` self "UpdatePlayerPositionOnMap" (`self.InAirUpdateRate`) true :!label _label))
  (set `self.UpdateTimerHandle` _returnvalue))

(event `OnPlayerJump`
  (set `self.Jumping?` true)
  (if (`self.Visible?`)
    (goto _label)))

(event `OnPlayerLand`
  (bind _updatetimerhandle (`self.UpdateTimerHandle`))
  (set `self.Jumping?` false)
  (if (`KismetSystemLibrary.K2_IsValidTimerHandle` _updatetimerhandle)
    (`KismetSystemLibrary.K2_ClearAndInvalidateTimerHandle` _updatetimerhandle)
    (`self.UpdatePlayerPositionOnMap`)))

(event `OnInputModifySize`
  (params (`Increase?` :type Boolean) (Percent :type Integer))
  (bind _mapreference (`self.MapReference`))
  (if (`self.Visible?`)
    (`self.ModifyMapSize` (+ (* (`KismetMathLibrary.Conv_IntToDouble` (`KismetMathLibrary.SelectInt` 1 -1 `Increase?`)) (/ (`KismetMathLibrary.Conv_IntToDouble` (`KismetMathLibrary.Clamp` Percent 0 100)) 100.0)) 1.0))
    (if (not `Increase?`)
      (`Widget.SetRenderTranslation` (`/Game/WorldMapAssets/Widgets/W_WorldMap.MapOverlay` _mapreference) (* (`.Translation` (break `WidgetTransform` (`Widget.RenderTransform` _mapreference))) (`self.CurrentSizeMultiplier`))))))

(event `OnMapClick`
  (params (Position :type "Vector2D Structure"))
  (bind _out (`self.TraceDownWorldLocation` (`self.MapPositionToWorldLocation` Position)))
  (`/Engine/EditorBlueprintResources/StandardMacros.CompareInt` (`self.MaxNumberOfMarkers`)
    (:`>`
      (if (>= (`KismetArrayLibrary.Array_Length` (`self.CurrentMarkers`)) (`self.MaxNumberOfMarkers`))
        (`self.RemoveMarkerByIndex` 0)))
    (:`<`
      _))
  (bind _returnvalue (`|SpawnActorFromClass` "/Game/WorldMapAssets/Actors/BP_Marker.BP_Marker_C" (`KismetMathLibrary.MakeTransform` _out) "Undefined" "OverrideRootScale" null null))
  (bind _markercolour (`self.SelectMarkerColour`))
  (`self.AddMarker` (make `/Game/WorldMapAssets/Structures/S_MarkerInfo` _markercolour _returnvalue null _out)))

(fn `AddMarker`
  (params (Marker :type "/Game/WorldMapAssets/Structures/S_MarkerInfo Structure"))
  (locals (LocalIndex :type Integer :default 0))
  (bind ((`Colour_8_A4FDA0874BB3CCC363A7838322AF7DD5` _colour) (`WorldLocation_2_918652674AA0A92091F71184CB699CA3` _worldlocation)) (break `/Game/WorldMapAssets/Structures/S_MarkerInfo` Marker))
  (bind _markersize (`self.MarkerSize`))
  (bind _returnvalue (`KismetArrayLibrary.Array_Add` (`self.CurrentMarkers`) Marker))
  (bind _output_get (set `local.LocalIndex` _returnvalue))
  (bind _widget (`/Game/WorldMapAssets/Widgets/W_WorldMap.AddMarkerToMap` (`self.MapReference`) _output_get self _colour (`self.LocationToMapPosition` _worldlocation (`KismetMathLibrary.MakeVector2D` (`KismetMathLibrary.Conv_IntToDouble` _markersize) (`KismetMathLibrary.Conv_IntToDouble` _markersize)))))
  (setmembers `/Game/WorldMapAssets/Structures/S_MarkerInfo` :`StructRef` (`|GetArrayItem` (`self.CurrentMarkers`) (`local.LocalIndex`)) :`Widget` _widget)
  (return))

(fn `ConvertLocationToMapLocation`
  (params (Location :type "Vector Structure"))
  (returns (MapLocation :type "Vector2D Structure"))
  (bind _returnvalue_x (`KismetMathLibrary.BreakVector` (`Actor.K2_GetActorLocation` (`self.UpperLeftCorner`))))
  (bind (_returnvalue_x_2 _returnvalue_y) (`KismetMathLibrary.BreakVector` (`Actor.K2_GetActorLocation` (`self.UpperLeftCorner`))))
  (return (`KismetMathLibrary.MakeVector2D` (`KismetMathLibrary.Abs` (- Location_Y _returnvalue_y)) (`KismetMathLibrary.Abs` (- Location_X _returnvalue_x)))))

(fn `GetMapHeight`
  (returns (MapHeight :type "Float (double-precision)"))
  (bind _returnvalue_x (`KismetMathLibrary.BreakVector` (`Actor.K2_GetActorLocation` (`self.LowerRightCorner`))))
  (bind _returnvalue_x_2 (`KismetMathLibrary.BreakVector` (`Actor.K2_GetActorLocation` (`self.UpperLeftCorner`))))
  (return (`KismetMathLibrary.Abs` (- _returnvalue_x _returnvalue_x_2))))

(fn `GetMapWidth`
  (returns (MapWidth :type "Float (double-precision)"))
  (bind (_returnvalue_x _returnvalue_y) (`KismetMathLibrary.BreakVector` (`Actor.K2_GetActorLocation` (`self.LowerRightCorner`))))
  (bind (_returnvalue_x_2 _returnvalue_y_2) (`KismetMathLibrary.BreakVector` (`Actor.K2_GetActorLocation` (`self.UpperLeftCorner`))))
  (return (`KismetMathLibrary.Abs` (- _returnvalue_y _returnvalue_y_2))))

(fn `LocationToMapPosition`
  (params (Location :type "Vector Structure") (WidgetSize :type "Vector2D Structure"))
  (returns (WidgetLocation :type "Vector2D Structure"))
  (bind (_maplocation_x _maplocation_y) (`KismetMathLibrary.BreakVector2D` (`self.ConvertLocationToMapLocation` Location)))
  (return (`KismetMathLibrary.MakeVector2D` (- (* (/ _maplocation_x (`self.GetMapWidth`)) (`KismetMathLibrary.Conv_IntToDouble` (`/Game/WorldMapAssets/Widgets/W_WorldMap.MapSizeX` (`self.MapReference`)))) (/ WidgetSize_X 2.0)) (- (* (/ _maplocation_y (`self.GetMapHeight`)) (`KismetMathLibrary.Conv_IntToDouble` (`/Game/WorldMapAssets/Widgets/W_WorldMap.MapSizeY` (`self.MapReference`)))) (/ WidgetSize_Y 2.0)))))

(fn `MapOutOfBoundaries?`
  (returns (`Out?` :type Boolean))
  (bind (_returnvalue_x _returnvalue_y) (`KismetMathLibrary.BreakVector2D` (`WidgetLayoutLibrary.GetViewportSize`)))
  (bind (_returnvalue_x_2 _returnvalue_y_2) (`KismetMathLibrary.BreakVector2D` (`Widget.GetDesiredSize` (`self.MapReference`))))
  (return (or (> _returnvalue_x_2 _returnvalue_x) (> _returnvalue_y_2 _returnvalue_y))))

(fn `MapPositionToWorldLocation`
  (params (Position :type "Vector2D Structure"))
  (returns (Location :type "Vector Structure"))
  (locals (LocalPercentageInX :type "Float (double-precision)" :default 0.0) (LocalPercentageInY :type "Float (double-precision)" :default 0.0))
  (bind (_returnvalue_x _returnvalue_y) (`KismetMathLibrary.BreakVector` (`Actor.K2_GetActorLocation` (`self.UpperLeftCorner`))))
  (set `local.LocalPercentageInX` (/ Position_X (`KismetMathLibrary.Conv_IntToDouble` (`/Game/WorldMapAssets/Widgets/W_WorldMap.MapSizeY` (`self.MapReference`)))))
  (set `local.LocalPercentageInY` (/ Position_Y (`KismetMathLibrary.Conv_IntToDouble` (`/Game/WorldMapAssets/Widgets/W_WorldMap.MapSizeX` (`self.MapReference`)))))
  (return (`KismetMathLibrary.MakeVector` (- _returnvalue_x (* (`self.GetMapHeight`) (`local.LocalPercentageInY`))) (+ _returnvalue_y (* (`self.GetMapWidth`) (`local.LocalPercentageInX`))))))

(fn `ModifyMapSize`
  (params (Multiplier :type "Float (double-precision)"))
  (bind (_returnvalue_x _returnvalue_y) (`KismetMathLibrary.BreakVector2D` (* (`self.OriginalPlayerSize`) (`self.CurrentSizeMultiplier`))))
  (bind (_returnvalue_x_2 _returnvalue_y_2) (`KismetMathLibrary.BreakVector2D` (* (`self.OriginalMapSize`) (`self.CurrentSizeMultiplier`))))
  (if (>= Multiplier 0.0)
    (set `self.CurrentSizeMultiplier` (`KismetMathLibrary.FClamp` (* (`self.CurrentSizeMultiplier`) Multiplier) (`self.MinZoom`) (`self.MaxZoom`)))
    (`/Game/WorldMapAssets/Widgets/W_WorldMap.SetMapSize` (`self.MapReference`) (`KismetMathLibrary.Round` _returnvalue_x_2) (`KismetMathLibrary.Round` _returnvalue_y_2))
    (if (not (`self.KeepPlayerSizeWhenZooming?`))
      (`/Game/WorldMapAssets/Widgets/W_WorldMap.SetPlayerSize` (`self.MapReference`) (`KismetMathLibrary.Round` _returnvalue_x) (`KismetMathLibrary.Round` _returnvalue_y)))
    (`self.UpdatePlayerPositionOnMap`)
    (if (not (`self.KeepMarkerSizeWhenZooming?`))
      (set `self.MarkerSize` (`KismetMathLibrary.Round` (* (`self.OriginalMarkerSize`) (`self.CurrentSizeMultiplier`))))
      (`self.UpdateMarkerSizes`))
    (`self.UpdateMarkerPositions`)
    (return)
    (else
      (return))))

(fn `RemoveMarkerByIndex`
  (params (MarkerIndex :type Integer))
  (bind _currentmarkers (`self.CurrentMarkers`))
  (bind (_colour _markeractor _widget) (break `/Game/WorldMapAssets/Structures/S_MarkerInfo` (`|GetArrayItem` (`self.CurrentMarkers`) MarkerIndex)))
  (if (`KismetArrayLibrary.Array_IsValidIndex` (`self.CurrentMarkers`) MarkerIndex)
    (if (not (`KismetArrayLibrary.Array_Contains` (`self.AvailableColours`) _colour))
      (`KismetArrayLibrary.Array_Insert` (`self.AvailableColours`) _colour))
    (`Actor.K2_DestroyActor` _markeractor)
    (`Widget.RemoveFromParent` _widget)
    (`KismetArrayLibrary.Array_Remove` _currentmarkers MarkerIndex)
    (for (_array_element _array_index) _currentmarkers
      (bind ((`Widget_5_600DAE8243B0175AF8CD14A18D09D18E` _widget_2)) (break `/Game/WorldMapAssets/Structures/S_MarkerInfo` _array_element))
      (`/Engine/EditorBlueprintResources/StandardMacros.IsValid` _widget_2
        (:`Is Valid`
          (set `/Game/WorldMapAssets/Widgets/W_Marker.Index` _array_index _widget_2))))
    (return)
    (else
      (return))))

(fn `SelectMarkerColour`
  (returns (MarkerColour :type "LinearColor Structure"))
  (locals (LocalColour :type "LinearColor Structure"))
  (set `local.LocalColour` (`|GetArrayItem` (`self.AvailableColours`)))
  (`KismetArrayLibrary.Array_Remove` (`self.AvailableColours`))
  (if (<= (`KismetArrayLibrary.Array_Length` (`self.AvailableColours`)) 0)
    (set `self.AvailableColours` (`self.MarkerColours`)))
  (return (`local.LocalColour`)))

(fn `ShowMap`
  (params (`Show?` :type Boolean))
  (bind _returnvalue (`GameplayStatics.GetPlayerController` 0))
  (bind _returnvalue_2 (`GameplayStatics.GetPlayerController` 0))
  (if (!= `Show?` (`self.Visible?`))
    (bind _output_get (set `self.Visible?` `Show?`))
    (if _output_get
      (`Widget.SetVisibility` (`self.MapReference`) "Visible")
      (set `PlayerController.bShowMouseCursor` true _returnvalue_2)
      (`WidgetBlueprintLibrary.SetInputMode_GameAndUIEx` _returnvalue_2 (`self.MainReference`) "DoNotLock" false)
      (`self.UpdatePlayerPositionOnMap`)
      (return)
      (else
        (`Widget.SetVisibility` (`self.MapReference`) "Hidden")
        (set `PlayerController.bShowMouseCursor` false _returnvalue)
        (`WidgetBlueprintLibrary.SetInputMode_GameOnly` _returnvalue)
        (return)))
    (else
      (return))))

(fn `ToggleVisibility`
  (bind _visible_ (`self.Visible?`))
  (`self.ShowMap` (not _visible_))
  (if (and _visible_ (`self.Jumping?`))
    (`self.StartTimer`)
    (return)
    (elif (and (not (`self.Visible?`)) (`KismetSystemLibrary.K2_IsValidTimerHandle` (`self.UpdateTimerHandle`)))
      (`KismetSystemLibrary.K2_ClearAndInvalidateTimerHandle` (`self.UpdateTimerHandle`))
      (return)
      (else
        (return)))))

(fn `TraceDownWorldLocation`
  (params (In :type "Vector Structure"))
  (returns (Out :type "Vector Structure"))
  (locals (LocalIn :type "Vector Structure"))
  (bind (_localin_x _localin_y) (`KismetMathLibrary.BreakVector` (`local.LocalIn`)))
  (set `local.LocalIn` In)
  (bind (_outhit _returnvalue) (`KismetSystemLibrary.LineTraceSingle` (`KismetMathLibrary.MakeVector` _localin_x _localin_y (`self.TraceDownHeight`)) (`local.LocalIn`) "TraceTypeQuery1"))
  (if _returnvalue
    (return (`.Location` (`GameplayStatics.BreakHitResult` _outhit)))
    (else
      (return (`local.LocalIn`)))))

(fn `UpdateMarkerPositions`
  (bind _markersize (`self.MarkerSize`))
  (for _array_element (`self.CurrentMarkers`)
    (bind (_colour _markeractor _widget _worldlocation) (break `/Game/WorldMapAssets/Structures/S_MarkerInfo` _array_element))
    (`/Engine/EditorBlueprintResources/StandardMacros.IsValid` _widget
      (:`Is Valid`
        (`Widget.SetRenderTranslation` _widget (`self.LocationToMapPosition` _worldlocation (`KismetMathLibrary.MakeVector2D` (`KismetMathLibrary.Conv_IntToDouble` _markersize) (`KismetMathLibrary.Conv_IntToDouble` _markersize)))))))
  (return))

(fn `UpdateMarkerSizes`
  (for _array_element (`self.CurrentMarkers`)
    (bind (_colour _markeractor _widget) (break `/Game/WorldMapAssets/Structures/S_MarkerInfo` _array_element))
    (`/Engine/EditorBlueprintResources/StandardMacros.IsValid` _widget
      (:`Is Valid`
        (`/Game/WorldMapAssets/Widgets/W_Marker.UpdateSize` _widget (`self.MarkerSize`)))))
  (return))

(fn `UpdatePlayerPositionOnMap`
  (bind _originalplayersize (`self.OriginalPlayerSize`))
  (`Widget.SetRenderTranslation` (`/Game/WorldMapAssets/Widgets/W_WorldMap.PlayerBox` (`self.MapReference`)) (`self.LocationToMapPosition` (`Actor.K2_GetActorLocation` (`self.Player`)) (select `bool` (`self.KeepPlayerSizeWhenZooming?`) :`false` (* _originalplayersize (`self.CurrentSizeMultiplier`)) :`true` _originalplayersize)))
  (return))