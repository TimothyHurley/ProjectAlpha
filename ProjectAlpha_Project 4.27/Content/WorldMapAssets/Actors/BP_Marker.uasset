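; BP_Marker is a world map marker actor with a discovery sphere and an optional smoke particle effect.
; On BeginPlay it sizes the sphere from a minimum radius and a multiplier, and sets particle visibility from the ShowSmoke flag.
; When an overlapping actor has a capsule component, it only prints a placeholder debug string, with no discovery logic in this Blueprint.
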(event `self.ReceiveBeginPlay`
  (`SphereComponent.SetSphereRadius` (`self.DiscoverSphere`) (* (`self.MinRadius`) (`self.RadiusMultiplier`)) false)
  (`SceneComponent.SetVisibility` (`self.ParticleSystem`) (`self.ShowSmoke?`) false))

(event `self.DiscoverSphere.OnComponentBeginOverlap`
  (params (OverlappedComponent :type "PrimitiveComponent Object Reference") (OtherActor :type "Actor Object Reference") (OtherComp :type "PrimitiveComponent Object Reference") (OtherBodyIndex :type Integer) (bFromSweep :type Boolean) (SweepResult :type "HitResult Structure (by ref)"))
  (`/Engine/EditorBlueprintResources/StandardMacros.IsValid` (`self.GetComponentByClass` OtherActor "/Script/Engine.CapsuleComponent")
    (:`Is Valid`
      (`KismetSystemLibrary.PrintString` "Yada" true true (struct :`G` 1.0 :`B` 1.0 :`A` 1.0) 5.0))))

(fn `UserConstructionScript`)