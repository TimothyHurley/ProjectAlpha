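; DeathBox is a kill volume that ends the player's run and restarts the current level on contact.
; On actor overlap it filters for the player, calls Death on the ThirdPersonCharacter and prints a taunting message.
; It then fades the camera to a held, partly opaque red, waits a configurable delay and reopens the current level by name.
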(event `self.ReceiveActorBeginOverlap`
  (params (OtherActor :type "Actor Object Reference"))
  (`/Game/PrototypeAssets/MacroLibrary/Main.IsPlayer` OtherActor
    (:`Is Player`
      (bind _asthird_person_character (cast `/Game/ThirdPersonBP/Blueprints/ThirdPersonCharacter` OtherActor))
      (`/Game/ThirdPersonBP/Blueprints/ThirdPersonCharacter.Death` _asthird_person_character)
      (`KismetSystemLibrary.PrintString` "You ded, therefore you succ")
      (`PlayerCameraManager.StartCameraFade` (`GameplayStatics.GetPlayerCameraManager` 0) 0.0 0.6 0.2 (struct :`R` 1.0 :`A` 1.0) false true)
      (`KismetSystemLibrary.Delay` (`self.Delay duration`))
      (bind _returnvalue (`GameplayStatics.GetCurrentLevelName` true))
      (`GameplayStatics.OpenLevel` (`KismetStringLibrary.Conv_StringToName` _returnvalue)))))

(fn `UserConstructionScript`)