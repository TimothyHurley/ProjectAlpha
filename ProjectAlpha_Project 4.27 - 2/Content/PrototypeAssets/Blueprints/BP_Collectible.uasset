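; BP_Collectible is a pickup actor that flies into the player and disappears when the player overlaps it.
; On overlap it caches its location and plays a timeline, whose Collection track drives movement and shrinking.
; Movement lerps from the cached start to the player pawn's live location, while scale lerps from its current value toward a small size each update.
; The actor destroys itself when the timeline finishes.
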(event `self.ReceiveBeginPlay`)

(event `self.ReceiveActorBeginOverlap`
  (params (OtherActor :type "Actor Object Reference"))
  (`/Game/PrototypeAssets/MacroLibrary/Main.IsPlayer` OtherActor
    (:`Is Player`
      (`self.GetActorLocation`)
      (bind (_direction _collection) (`Timeline|Timeline_0`)
        (:`Update`
          (`self.Move to Player` (`self.Lerp start Location`) _collection)
          (`self.ShrinkActor` _collection))
        (:`Finished`
          (`self.K2_DestroyActor`))))))

(fn `GetActorLocation`
  (set `self.Lerp start Location` (`self.K2_GetActorLocation`)))

(fn `Move to Player`
  (params (A :type "Vector Structure") (Alpha :type "Float (double-precision)"))
  (`self.K2_SetActorLocation` (`KismetMathLibrary.VLerp` A (`self.K2_GetActorLocation` (`GameplayStatics.GetPlayerPawn` 0)) Alpha)))

(fn `ShrinkActor`
  (params (Alpha :type "Float (double-precision)"))
  (`self.SetActorScale3D` (`KismetMathLibrary.VLerp` (`self.GetActorScale3D`) (0.1 0.1 0.1) Alpha)))

(fn `UserConstructionScript`)