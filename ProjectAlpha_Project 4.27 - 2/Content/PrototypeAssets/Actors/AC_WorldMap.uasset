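; World map component that shows the player, undiscovered areas and player-placed markers on a toggleable, zoomable UI map.
; TopLeft and BottomRight bounds actors drive conversion between world locations and map positions.
; Map clicks alternate between previewing a downward-traced spot and spawning a colour-coded A_MapMarker, evicting the oldest at the limit.
; The player icon updates on movement or by timer while airborne, and discovered areas lose their circles.
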(event `InitializeMap`
  (params (Player :type "Character Object Reference"))
  (bind _worldmapref (`self.WorldMapRef`))
  (bind _worldmapref_2 (`self.WorldMapRef`))
  (`/Engine/EditorBlueprintResources/StandardMacros.IsValid` Player
    (:`Is Valid`
      (set `self.Player` Player)
      (bind _returnvalue (`|CreateWidget` "/Game/PrototypeAssets/Widgets/W_MainPanel.W_MainPanel_C"))
      (bind _output_get (set `self.MainPanelRef` _returnvalue))
      (bind _output_get_2 (set `self.WorldMapRef` (`/Game/PrototypeAssets/Widgets/W_MainPanel.W_WorldMap` _output_get)))
      (`/Game/PrototypeAssets/Widgets/W_WorldMap.Initialize` _output_get_2 self)
      (set `self.OriginalPlayerIconSize` (`KismetMathLibrary.MakeVector2D` (`KismetMathLibrary.Conv_IntToDouble` (`/Game/PrototypeAssets/Widgets/W_WorldMap.PlayerSizeX` _worldmapref)) (`KismetMathLibrary.Conv_IntToDouble` (`/Game/PrototypeAssets/Widgets/W_WorldMap.PlayerSizeY` _worldmapref))))
      (set `self.OriginalMapSize` (`KismetMathLibrary.MakeVector2D` (`KismetMathLibrary.Conv_IntToDouble` (`/Game/PrototypeAssets/Widgets/W_WorldMap.MapSizeX` _worldmapref_2)) (`KismetMathLibrary.Conv_IntToDouble` (`/Game/PrototypeAssets/Widgets/W_WorldMap.MapSizeY` _worldmapref_2))))
      (set `self.OriginalMapMarkerSize` (`self.MapMarkerSize`))
      (set `self.AvailableMarkerColours` (`self.MarkerColours`))
      (bind _outactors (`GameplayStatics.GetAllActorsOfClass` "/Game/PrototypeAssets/Actors/A_UndiscoveredArea.A_UndiscoveredArea_C"))
      (bind _output_get_3 (set `self.UndiscoveredAreaRefs` _outactors))
      (for _array_element _output_get_3
        (bind _size (`self.AreaRadiusToMapCircleSize` _array_element))
        (bind _out (`/Game/PrototypeAssets/Widgets/W_WorldMap.AddAreaToMap` (`self.WorldMapRef`) _size (`self.LocationToMapPosition` (`Actor.K2_GetActorLocation` _array_element) (`KismetMathLibrary.MakeVector2D` _size _size))))
        (`KismetArrayLibrary.Array_Add` (`self.UndiscoveredAreaWidgetRefs`) _out))
      (`self.ShowMap` false)
      (`UserWidget.AddToViewport` (`self.MainPanelRef`) 0))
    (:`Is Not Valid`
      (`KismetSystemLibrary.PrintString` "Error: Player is not valid" true true (struct :`R` 1.0 :`A` 1.0) 3.0))))

(event `OnPlayerMove`
  (if (`self.IsVisible?`)
    (`self.UpdatePlayerPositionOnMap`)))

(event `StartTimer`
  (bind _returnvalue (`KismetSystemLibrary.K2_SetTimer` self "UpdatePlayerPositionOnMap" (`self.InAirUpdateRate`) true :!label _label))
  (set `self.UpdateTimerHandle` _returnvalue))

(event `OnPlayerJump`
  (set `self.IsJumping?` true)
  (if (`self.IsVisible?`)
    (goto _label)))

(event `OnPlayerLand`
  (bind _updatetimerhandle (`self.UpdateTimerHandle`))
  (set `self.IsJumping?` false)
  (if (`KismetSystemLibrary.K2_IsValidTimerHandle` _updatetimerhandle)
    (`KismetSystemLibrary.K2_ClearAndInvalidateTimerHandle` _updatetimerhandle)
    (`self.UpdatePlayerPositionOnMap`)))

(event `OnInputModifySize`
  (params (`Increase?` :type Boolean) (Percent :type Integer))
  (bind _worldmapref (`self.WorldMapRef`))
  (if (`self.IsVisible?`)
    (`self.ModifyMapSize` (+ (* (`KismetMathLibrary.Conv_IntToDouble` (`KismetMathLibrary.SelectInt` 1 -1 `Increase?`)) (/ (`KismetMathLibrary.Conv_IntToDouble` (`KismetMathLibrary.Clamp` Percent 0 100)) 100.0)) 1.0))
    (if (not `Increase?`)
      (`Widget.SetRenderTranslation` (`/Game/PrototypeAssets/Widgets/W_WorldMap.Overlay_WorldMap` _worldmapref) (* (`.Translation` (break `WidgetTransform` (`Widget.RenderTransform` _worldmapref))) (`self.CurrentSizeMultiplier`))))))

(event `OnMapClick`
  (params (Position :type "Vector2D Structure"))
  (bind _mapmarkersize (`self.MapMarkerSize`))
  (bind _out (`self.TraceDownWorldLocation` (`self.MapPositionToWorldLocation` Position)))
  (`/Engine/EditorBlueprintResources/StandardMacros.CompareInt` (`self.MaxNumberOfMarkers`)
    (:`>`
      _)
    (:`<`
      _))
  (`/Engine/EditorBlueprintResources/StandardMacros.FlipFlop`
    (:`A`
      (set `self.LocationOfMarkerPreview` _out)
      (bind (_marker _slider) (`/Game/PrototypeAssets/Widgets/W_WorldMap.AddMarkerPreviewToMap` (`self.WorldMapRef`) self (`self.LocationToMapPosition` _out (`KismetMathLibrary.MakeVector2D` (`KismetMathLibrary.Conv_IntToDouble` _mapmarkersize) (`KismetMathLibrary.Conv_IntToDouble` _mapmarkersize))))))
    (:`B`
      (bind _returnvalue (`|SpawnActorFromClass` :`Class` "/Game/PrototypeAssets/Actors/A_MapMarker.A_MapMarker_C" :`SpawnTransform` (`KismetMathLibrary.MakeTransform` (`self.LocationOfMarkerPreview`)) :`CollisionHandlingOverride` "Undefined" :`TransformScaleMethod` "OverrideRootScale" :`RadiusMultiplier` (`self.MapCircleSizeToAreaRadius` (`self.MapMarkerSize`)) :`WorldMapRef` null :`Instigator` null))
      (bind _markercolour (`self.SelectMarkerColour`))
      (`self.AddMarker` (make `/Game/PrototypeAssets/Structures/S_MapMarkers` _markercolour _returnvalue (`self.MapMarkerSize`) null (`self.LocationOfMarkerPreview`)))
      (`Widget.RemoveFromParent` _slider)
      (`Widget.RemoveFromParent` _marker)
      (set `self.MapMarkerSize` (`self.OriginalMapMarkerSize`))
      (`/Engine/EditorBlueprintResources/StandardMacros.CompareInt` (`self.MaxNumberOfMarkers`)
        (:`>`
          (if (>= (`KismetArrayLibrary.Array_Length` (`self.MapMarkerRefs`)) (`self.MaxNumberOfMarkers`))
            (`self.RemoveMarkerByIndex` 0)))))))

(event `OnDiscoverArea`
  (params (Area :type "/Game/PrototypeAssets/Actors/A_UndiscoveredArea Object Reference"))
  (bind _undiscoveredarearefs (`self.UndiscoveredAreaRefs`))
  (bind _output (`|GetArrayItem` (`self.UndiscoveredAreaWidgetRefs`) (`self.IndexOfUndiscoveredArea`)))
  (if (`KismetArrayLibrary.Array_Contains` (`self.UndiscoveredAreaRefs`) Area)
    (bind _output_get (set `self.IndexOfUndiscoveredArea` (`KismetArrayLibrary.Array_Find` _undiscoveredarearefs Area)))
    (`KismetArrayLibrary.Array_Remove` _undiscoveredarearefs _output_get)
    (`/Engine/EditorBlueprintResources/StandardMacros.IsValid` _output
      (:`Is Valid`
        (`/Game/PrototypeAssets/Widgets/W_UndiscoveredArea.RemoveWidget` _output)
        (`KismetArrayLibrary.Array_Remove` (`self.UndiscoveredAreaWidgetRefs`) (`self.IndexOfUndiscoveredArea`)))
      (:`Is Not Valid`
        _))
    (`/Game/PrototypeAssets/Actors/A_UndiscoveredArea.OnDiscover` Area)))

(fn `AddMarker`
  (params (Marker :type "/Game/PrototypeAssets/Structures/S_MapMarkers Structure"))
  (locals (LocalIndex :type Integer :default 0))
  (bind ((`Colour_8_A4FDA0874BB3CCC363A7838322AF7DD5` _colour) (`MarkerSize_14_D4E4E9014C4313BECD0BD3B7C811129D` _markersize) (`WorldLocation_2_918652674AA0A92091F71184CB699CA3` _worldlocation)) (break `/Game/PrototypeAssets/Structures/S_MapMarkers` Marker))
  (bind _mapmarkersize (`self.MapMarkerSize`))
  (bind _returnvalue (`KismetArrayLibrary.Array_Add` (`self.MapMarkerRefs`) Marker))
  (bind _output_get (set `local.LocalIndex` _returnvalue))
  (bind _widget (`/Game/PrototypeAssets/Widgets/W_WorldMap.AddMarkerToMap` (`self.WorldMapRef`) _output_get self _colour (`self.LocationToMapPosition` _worldlocation (`KismetMathLibrary.MakeVector2D` (`KismetMathLibrary.Conv_IntToDouble` _mapmarkersize) (`KismetMathLibrary.Conv_IntToDouble` _mapmarkersize)))))
  (setmembers `/Game/PrototypeAssets/Structures/S_MapMarkers` :`StructRef` (`|GetArrayItem` (`self.MapMarkerRefs`) (`local.LocalIndex`)) :`Widget` _widget)
  (return))

(fn `AreaRadiusToMapCircleSize`
  (params (Area :type "/Game/PrototypeAssets/Actors/A_UndiscoveredArea Object Reference"))
  (returns (Size :type "Float (double-precision)"))
  (return (* (`/Game/PrototypeAssets/Widgets/W_WorldMap.MapSizeX` (`self.WorldMapRef`)) (/ (* (`/Game/PrototypeAssets/Actors/A_UndiscoveredArea.AreaRadius` Area) 2.0) (`self.GetMapWidth`)))))

(fn `ConvertLocationToMapLocation`
  (params (Location :type "Vector Structure"))
  (returns (MapLocation :type "Vector2D Structure"))
  (bind _returnvalue_x (`KismetMathLibrary.BreakVector` (`Actor.K2_GetActorLocation` (`self.TopLeft`))))
  (bind (_returnvalue_x_2 _returnvalue_y) (`KismetMathLibrary.BreakVector` (`Actor.K2_GetActorLocation` (`self.TopLeft`))))
  (return (`KismetMathLibrary.MakeVector2D` (`KismetMathLibrary.Abs` (- Location_Y _returnvalue_y)) (`KismetMathLibrary.Abs` (- Location_X _returnvalue_x)))))

(fn `GetMapHeight`
  (returns (MapHeight :type "Float (double-precision)"))
  (bind _returnvalue_x (`KismetMathLibrary.BreakVector` (`Actor.K2_GetActorLocation` (`self.BottomRight`))))
  (bind _returnvalue_x_2 (`KismetMathLibrary.BreakVector` (`Actor.K2_GetActorLocation` (`self.TopLeft`))))
  (return (`KismetMathLibrary.Abs` (- _returnvalue_x _returnvalue_x_2))))

(fn `GetMapWidth`
  (returns (MapWidth :type "Float (double-precision)"))
  (bind (_returnvalue_x _returnvalue_y) (`KismetMathLibrary.BreakVector` (`Actor.K2_GetActorLocation` (`self.BottomRight`))))
  (bind (_returnvalue_x_2 _returnvalue_y_2) (`KismetMathLibrary.BreakVector` (`Actor.K2_GetActorLocation` (`self.TopLeft`))))
  (return (`KismetMathLibrary.Abs` (- _returnvalue_y _returnvalue_y_2))))

(fn `LocationToMapPosition`
  (params (Location :type "Vector Structure") (WidgetSize :type "Vector2D Structure"))
  (returns (WidgetLocation :type "Vector2D Structure"))
  (bind (_maplocation_x _maplocation_y) (`KismetMathLibrary.BreakVector2D` (`self.ConvertLocationToMapLocation` Location)))
  (return (`KismetMathLibrary.MakeVector2D` (- (* (/ _maplocation_x (`self.GetMapWidth`)) (`KismetMathLibrary.Conv_IntToDouble` (`/Game/PrototypeAssets/Widgets/W_WorldMap.MapSizeX` (`self.WorldMapRef`)))) (/ WidgetSize_X 2.0)) (- (* (/ _maplocation_y (`self.GetMapHeight`)) (`KismetMathLibrary.Conv_IntToDouble` (`/Game/PrototypeAssets/Widgets/W_WorldMap.MapSizeY` (`self.WorldMapRef`)))) (/ WidgetSize_Y 2.0)))))

(fn `MapCircleSizeToAreaRadius`
  (params (MarkerSize :type Integer))
  (returns (NewDiscoverRadius :type "Float (double-precision)"))
  (locals (MinMultiplier :type "Float (double-precision)" :default 1.0) (MaxMultiplier :type "Float (double-precision)" :default 8.0))
  (return (/ (`KismetMathLibrary.Conv_IntToDouble` (* MarkerSize 100)) (`KismetMathLibrary.Conv_IntToDouble` (* (`self.OriginalMapMarkerSize`) 100)))))

(fn `MapOutOfBoundaries?`
  (returns (`Out?` :type Boolean))
  (bind (_returnvalue_x _returnvalue_y) (`KismetMathLibrary.BreakVector2D` (`WidgetLayoutLibrary.GetViewportSize`)))
  (bind (_returnvalue_x_2 _returnvalue_y_2) (`KismetMathLibrary.BreakVector2D` (`Widget.GetDesiredSize` (`self.WorldMapRef`))))
  (return (or (> _returnvalue_x_2 _returnvalue_x) (> _returnvalue_y_2 _returnvalue_y))))

(fn `MapPositionToWorldLocation`
  (params (Position :type "Vector2D Structure"))
  (returns (Location :type "Vector Structure"))
  (locals (LocalPercentageInX :type "Float (double-precision)" :default 0.0) (LocalPercentageInY :type "Float (double-precision)" :default 0.0))
  (bind (_returnvalue_x _returnvalue_y) (`KismetMathLibrary.BreakVector` (`Actor.K2_GetActorLocation` (`self.TopLeft`))))
  (set `self.MapPercentageX` (/ Position_X (`KismetMathLibrary.Conv_IntToDouble` (`/Game/PrototypeAssets/Widgets/W_WorldMap.MapSizeY` (`self.WorldMapRef`)))))
  (set `self.MapPercentageY` (/ Position_Y (`KismetMathLibrary.Conv_IntToDouble` (`/Game/PrototypeAssets/Widgets/W_WorldMap.MapSizeX` (`self.WorldMapRef`)))))
  (return (`KismetMathLibrary.MakeVector` (- _returnvalue_x (* (`self.GetMapHeight`) (`self.MapPercentageY`))) (+ _returnvalue_y (* (`self.GetMapWidth`) (`self.MapPercentageX`))))))

(fn `ModifyMapSize`
  (params (Multiplier :type "Float (double-precision)"))
  (bind (_returnvalue_x _returnvalue_y) (`KismetMathLibrary.BreakVector2D` (* (`self.OriginalPlayerIconSize`) (`self.CurrentSizeMultiplier`))))
  (bind (_returnvalue_x_2 _returnvalue_y_2) (`KismetMathLibrary.BreakVector2D` (* (`self.OriginalMapSize`) (`self.CurrentSizeMultiplier`))))
  (if (>= Multiplier 0.0)
    (set `self.CurrentSizeMultiplier` (`KismetMathLibrary.FClamp` (* (`self.CurrentSizeMultiplier`) Multiplier) (`self.MinZoom`) (`self.MaxZoom`)))
    (`/Game/PrototypeAssets/Widgets/W_WorldMap.SetMapSize` (`self.WorldMapRef`) (`KismetMathLibrary.Round` _returnvalue_x_2) (`KismetMathLibrary.Round` _returnvalue_y_2))
    (if (not (`self.KeepPlayerSizeWhenZooming?`))
      (`/Game/PrototypeAssets/Widgets/W_WorldMap.SetPlayerIconSize` (`self.WorldMapRef`) (`KismetMathLibrary.Round` _returnvalue_x) (`KismetMathLibrary.Round` _returnvalue_y)))
    (`self.UpdatePlayerPositionOnMap`)
    (if (not (`self.KeepMarkerSizeWhenZooming?`))
      (set `self.MapMarkerSize` (`KismetMathLibrary.Round` (* (`self.OriginalMapMarkerSize`) (`self.CurrentSizeMultiplier`))))
      (`self.UpdateMarkerSizes`))
    (`self.UpdateMarkerPositions`)
    (`self.UpdateAreaSizesAndPositions`)
    (return)
    (else
      (return))))

(fn `RemoveMarkerByIndex`
  (params (MarkerIndex :type Integer))
  (bind _mapmarkerrefs (`self.MapMarkerRefs`))
  (bind (_colour _markeractor _markersize _widget) (break `/Game/PrototypeAssets/Structures/S_MapMarkers` (`|GetArrayItem` (`self.MapMarkerRefs`) MarkerIndex)))
  (if (`KismetArrayLibrary.Array_IsValidIndex` (`self.MapMarkerRefs`) MarkerIndex)
    (if (not (`KismetArrayLibrary.Array_Contains` (`self.AvailableMarkerColours`) _colour))
      (`KismetArrayLibrary.Array_Add` (`self.AvailableMarkerColours`) _colour))
    (`Actor.K2_DestroyActor` _markeractor)
    (`Widget.RemoveFromParent` _widget)
    (`KismetArrayLibrary.Array_Remove` _mapmarkerrefs MarkerIndex)
    (for (_array_element _array_index) _mapmarkerrefs
      (bind ((`MarkerSize_14_D4E4E9014C4313BECD0BD3B7C811129D` _markersize_2) (`Widget_5_600DAE8243B0175AF8CD14A18D09D18E` _widget_2)) (break `/Game/PrototypeAssets/Structures/S_MapMarkers` _array_element))
      (`/Engine/EditorBlueprintResources/StandardMacros.IsValid` _widget_2
        (:`Is Valid`
          (set `/Game/PrototypeAssets/Widgets/W_MapMarker.Index` _array_index _widget_2))))
    (return)
    (else
      (return))))

(fn `SelectMarkerColour`
  (returns (MarkerColour :type "LinearColor Structure"))
  (locals (LocalColour :type "LinearColor Structure"))
  (set `local.LocalColour` (`|GetArrayItem` (`self.AvailableMarkerColours`)))
  (`KismetArrayLibrary.Array_Remove` (`self.AvailableMarkerColours`))
  (if (== (- (`KismetArrayLibrary.Array_Length` (`self.MarkerColours`)) (`self.MaxNumberOfMarkers`)) (`KismetArrayLibrary.Array_Length` (`self.AvailableMarkerColours`)))
    (set `self.AvailableMarkerColours` (`self.MarkerColours`)))
  (return (`local.LocalColour`)))

(fn `ShowMap`
  (params (`Show?` :type Boolean))
  (bind _returnvalue (`GameplayStatics.GetPlayerController` 0))
  (bind _returnvalue_2 (`GameplayStatics.GetPlayerController` 0))
  (if (!= `Show?` (`self.IsVisible?`))
    (bind _output_get (set `self.IsVisible?` `Show?`))
    (if _output_get
      (`Widget.SetVisibility` (`self.WorldMapRef`) "Visible")
      (set `PlayerController.bShowMouseCursor` true _returnvalue_2)
      (`WidgetBlueprintLibrary.SetInputMode_GameAndUIEx` _returnvalue_2 (`self.MainPanelRef`) "DoNotLock" false)
      (`self.UpdatePlayerPositionOnMap`)
      (return)
      (else
        (`Widget.SetVisibility` (`self.WorldMapRef`) "Hidden")
        (set `PlayerController.bShowMouseCursor` false _returnvalue)
        (`WidgetBlueprintLibrary.SetInputMode_GameOnly` _returnvalue)
        (return)))
    (else
      (return))))

(fn `ToggleVisibility`
  (bind _isvisible_ (`self.IsVisible?`))
  (`self.ShowMap` (not _isvisible_))
  (if (and _isvisible_ (`self.IsJumping?`))
    (`self.StartTimer`)
    (return)
    (elif (and (not (`self.IsVisible?`)) (`KismetSystemLibrary.K2_IsValidTimerHandle` (`self.UpdateTimerHandle`)))
      (`KismetSystemLibrary.K2_ClearAndInvalidateTimerHandle` (`self.UpdateTimerHandle`))
      (return)
      (else
        (return)))))

(fn `TraceDownWorldLocation`
  (params (In :type "Vector Structure"))
  (returns (Out :type "Vector Structure"))
  (locals (LocalIn :type "Vector Structure"))
  (bind (_localin_x _localin_y) (`KismetMathLibrary.BreakVector` (`local.LocalIn`)))
  (set `local.LocalIn` In)
  (bind (_outhit _returnvalue) (`KismetSystemLibrary.LineTraceSingle` (`KismetMathLibrary.MakeVector` _localin_x _localin_y (`self.TraceDownHeight`)) (`local.LocalIn`) "TraceTypeQuery1"))
  (if _returnvalue
    (return (`.Location` (`GameplayStatics.BreakHitResult` _outhit)))
    (else
      (return (`local.LocalIn`)))))

(fn `UpdateAreaSizesAndPositions`
  (for (_array_element _array_index) (`self.UndiscoveredAreaRefs`)
    (bind _output (`|GetArrayItem` (`self.UndiscoveredAreaWidgetRefs`) _array_index))
    (`/Engine/EditorBlueprintResources/StandardMacros.IsValid` _output
      (:`Is Valid`
        (bind _size (`self.AreaRadiusToMapCircleSize` _array_element))
        (`/Game/PrototypeAssets/Widgets/W_UndiscoveredArea.UpdateCircleSize` _output _size)
        (`Widget.SetRenderTranslation` _output (`self.LocationToMapPosition` (`Actor.K2_GetActorLocation` _array_element) (`KismetMathLibrary.MakeVector2D` _size _size)))))))

(fn `UpdateMarkerPositions`
  (bind _mapmarkersize (`self.MapMarkerSize`))
  (for _array_element (`self.MapMarkerRefs`)
    (bind (_colour _markeractor _markersize _widget _worldlocation) (break `/Game/PrototypeAssets/Structures/S_MapMarkers` _array_element))
    (`/Engine/EditorBlueprintResources/StandardMacros.IsValid` _widget
      (:`Is Valid`
        (`Widget.SetRenderTranslation` _widget (`self.LocationToMapPosition` _worldlocation (`KismetMathLibrary.MakeVector2D` (`KismetMathLibrary.Conv_IntToDouble` _mapmarkersize) (`KismetMathLibrary.Conv_IntToDouble` _mapmarkersize)))))))
  (return))

(fn `UpdateMarkerSizes`
  (for _array_element (`self.MapMarkerRefs`)
    (bind (_colour _markeractor _markersize _widget) (break `/Game/PrototypeAssets/Structures/S_MapMarkers` _array_element))
    (`/Engine/EditorBlueprintResources/StandardMacros.IsValid` _widget
      (:`Is Valid`
        (`/Game/PrototypeAssets/Widgets/W_MapMarker.UpdateSize` _widget (`self.MapMarkerSize`)))))
  (return))

(fn `UpdatePlayerPositionOnMap`
  (bind _originalplayericonsize (`self.OriginalPlayerIconSize`))
  (`Widget.SetRenderTranslation` (`/Game/PrototypeAssets/Widgets/W_WorldMap.SizeBox_PlayerIcon` (`self.WorldMapRef`)) (`self.LocationToMapPosition` (`Actor.K2_GetActorLocation` (`self.Player`)) (select `bool` (`self.KeepPlayerSizeWhenZooming?`) :`false` (* _originalplayericonsize (`self.CurrentSizeMultiplier`)) :`true` _originalplayericonsize)))
  (return))